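; BP_Bullet is a platformer projectile that damages the player on contact.
; Each Tick moves it without sweep along its normalized local Direction by Speed per frame, unscaled by delta time, while a Delay destroys it after BulletLifetime.
; When SM_Bullet begins overlapping the player pawn cached on BeginPlay, it subtracts Damage directly from the character's Health and destroys itself.
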(event `self.ReceiveBeginPlay`
  ;[0.2356 0.4479 0.2707] Getting Player Reference
  (bind _asbp_third_person_character (cast `/Game/Platformer/BP_ThirdPersonCharacter` (`GameplayStatics.GetPlayerPawn` 0)))
  (set `self.PlayerReference` _asbp_third_person_character))

(event `self.ReceiveTick`
  (params (DeltaSeconds :type "Float (single-precision)"))
  ;[1 0.5566 0.1085] Bullet Movement
  (`self.K2_AddActorLocalOffset` (* (`KismetMathLibrary.Normal` (`self.Direction`)) (`self.Speed`)))
  ;[0.2836 0.1668 0.3906] Destroy Bullet After Elapsed Time
  (`KismetSystemLibrary.Delay` (`self.BulletLifetime`))
  (`self.K2_DestroyActor`))

(event `self.SM_Bullet.OnComponentBeginOverlap`
  (params (OverlappedComponent :type "PrimitiveComponent Object Reference") (OtherActor :type "Actor Object Reference") (OtherComp :type "PrimitiveComponent Object Reference") (OtherBodyIndex :type Integer) (bFromSweep :type Boolean) (SweepResult :type "HitResult Structure (by ref)"))
  ;[0.05387 0.25 0.215] Damage Player
  (if (== OtherActor (`self.PlayerReference`))
    (set `/Game/Platformer/BP_ThirdPersonCharacter.Health` (- (`/Game/Platformer/BP_ThirdPersonCharacter.Health` (`self.PlayerReference`)) (`self.Damage`)) (`self.PlayerReference`))
    ;[0.01747 0.009552 0.1927] Destroy Bullet
    (`self.K2_DestroyActor`)))

(fn `UserConstructionScript`)