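; Enemy turret for a platformer that fires BP_Bullet actors from its FiringPoint for as long as it exists.
; BeginPlay picks single or scatter fire; each mode re-calls itself after FiringDelay.
; Scatter shot spawns a volley of bullets, each with random yaw spread around the muzzle's facing.
; An optional Tick update turns the stem toward the player on the horizontal plane, setting the look-at as relative rotation.
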(event `self.ReceiveBeginPlay`
  ;[1 0.3345 0.7773] Type Of Shot
  (if (`self.UseScatterShot`)
    (`self.ScatterShot`)
    (else
      (`self.OneShot`))))

(event `self.ReceiveTick`
  (params (DeltaSeconds :type "Float (single-precision)"))
  (bind (_returnvalue_x _returnvalue_y) (`KismetMathLibrary.BreakVector` (`self.K2_GetActorLocation`)))
  (bind (_returnvalue_x_2 _returnvalue_y_2) (`KismetMathLibrary.BreakVector` (`self.K2_GetActorLocation` (`GameplayStatics.GetPlayerPawn` 0))))
  ;[0.2865 0.03595 0.08764] Look At Player
  (if (`self.LookAtPlayer`)
    (`SceneComponent.K2_SetRelativeRotation` (`self.SM_TurretStem`) (`KismetMathLibrary.FindLookAtRotation` (`KismetMathLibrary.MakeVector` _returnvalue_x _returnvalue_y) (`KismetMathLibrary.MakeVector` _returnvalue_x_2 _returnvalue_y_2)) false false)))

(event `OneShot`
  ;[0.3438 0.2463 0.1193] OneShot
  (`|SpawnActorFromClass` "/Game/Platformer/BP_Bullet.BP_Bullet_C" (`SceneComponent.GetSocketTransform` (`self.FiringPoint`) "None" "RTS_World") "Undefined" "MultiplyWithRoot" null null)
  ;[0.2225 0.276 0.02588] Recall One Shot
  (`KismetSystemLibrary.Delay` (`self.FiringDelay`))
  (`self.OneShot`))

(event `ScatterShot`
  (bind _returnvalue (`SceneComponent.GetSocketTransform` (`self.FiringPoint`) "None" "RTS_World"))
  ;[0.474 0.6133 1] ScatterShot
  (for _ (range 6)
    (`|SpawnActorFromClass` "/Game/Platformer/BP_Bullet.BP_Bullet_C" (`KismetMathLibrary.MakeTransform` (.location _returnvalue) (`KismetMathLibrary.MakeRotator` (.roll (.rotation _returnvalue)) (.pitch (.rotation _returnvalue)) (+ (.yaw (.rotation _returnvalue)) (`KismetMathLibrary.RandomFloatInRange` -30.0 30.0)))) "Undefined" "MultiplyWithRoot" null null))
  ;[0.2225 0.276 0.02588] Recall ScatterShot
  (`KismetSystemLibrary.Delay` (`self.FiringDelay`))
  (`self.ScatterShot`))

(fn `UserConstructionScript`)